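; HelpTrigger_BP is a trigger actor for Level 1 help that shows a Help_UI widget when the third-person player character overlaps it.
; Each qualifying overlap creates a new widget and adds it to the viewport, with no guard against repeats.
; A CheckCutScene function reports whether CutsceneToPlay is in the game instance's PlayedCutScenes, but the overlap logic does not call it.
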(event `self.ReceiveActorBeginOverlap`
  (params (OtherActor :type "Actor Object Reference"))
  (cast `/Game/ThirdPerson/Blueprints/BP_ThirdPersonCharacter` OtherActor)
  (bind _returnvalue (`|CreateWidget` "/Game/Special_Events/Level_1_Help/Help_UI.Help_UI_C"))
  (`UserWidget.AddToViewport` _returnvalue 0))

(fn `CheckCutScene`
  (returns (CutSceneAlreadyPlayed :type Boolean))
  (bind _asgame_instance_bp (cast `/Game/ThirdPerson/Blueprints/Save/GameInstance_BP` (`GameplayStatics.GetGameInstance`)))
  (return (`KismetArrayLibrary.Array_Contains` (`/Game/ThirdPerson/Blueprints/Save/GameInstance_BP.PlayedCutScenes` _asgame_instance_bp) (`self.Cutscene To Play`))))

(fn `UserConstructionScript`
  (`parent.UserConstructionScript`))