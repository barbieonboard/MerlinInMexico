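; LevelLoading_BP runs a timed screen fade when play begins, using the FadeInOut_UI widget.
; BeginPlay calls the FadeOut event, which creates the widget, stores it and adds it to the viewport.
; After a short delay it plays the widget's FadeIn animation in reverse at reduced speed, so one animation serves as the fade-out.
; A second delay then removes the widget from the screen.
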(event `self.ReceiveBeginPlay`
  (`self.FadeOut`))

(event `FadeOut`
  (bind _returnvalue (`|CreateWidget` "/Game/Special_Events/FadeInOut_UI.FadeInOut_UI_C"))
  (bind _output_get (set `self.UI` _returnvalue))
  (`UserWidget.AddToViewport` _output_get 0)
  (`KismetSystemLibrary.Delay` 2.0)
  (`UserWidget.PlayAnimationReverse` _returnvalue (`/Game/Special_Events/FadeInOut_UI.FadeIn` _returnvalue) 0.5 false)
  (`KismetSystemLibrary.Delay` 2.0)
  (`Widget.RemoveFromParent` (`self.UI`)))

(fn `UserConstructionScript`)